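; BP_GameState is a game state Blueprint that relays Lua state reload notifications to interested listeners.
; Objects register or unregister through subscriber events that maintain a listener list without duplicates.
; When OnLuaStateReloaded fires, it loops over that list and calls OnLuaStateReloaded on each listener, acting as a simple observer hub.
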(event `/Game/FunctionLibrary/BPI_EventDispatcher.AddSubscriberToLuaStateReload`
  (params (Listener :type "/Game/FunctionLibrary/BPI_EventListener Interface"))
  (`KismetArrayLibrary.Array_AddUnique` (`self.LuaStateListeners`) Listener))

(event `/Game/FunctionLibrary/BPI_EventDispatcher.RemoveSubscriberToLuaStateReload`
  (params (Listener :type "/Game/FunctionLibrary/BPI_EventListener Interface"))
  (if (`KismetArrayLibrary.Array_Contains` (`self.LuaStateListeners`) Listener)
    (`KismetArrayLibrary.Array_RemoveItem` (`self.LuaStateListeners`) Listener)))

(event `/Game/FunctionLibrary/BPI_EventListener.OnLuaStateReloaded`
  (for _array_element (`self.LuaStateListeners`)
    (`/Game/FunctionLibrary/BPI_EventListener.OnLuaStateReloaded` _array_element)))

(fn `UserConstructionScript`)