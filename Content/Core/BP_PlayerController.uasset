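; Player controller that spawns a cursor actor and drives the possessed character through Enhanced Input and interface messages.
; Tick sends a flattened character-to-cursor aim direction, while input handles movement, jumping, equipped-item actions and unequipping.
; Overlapping an equippable actor equips it automatically.
; A Lua state reload input broadcasts an event that re-reads the speed stat, which is stored but not yet applied.
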(event `self.ReceiveBeginPlay`
  (`parent.ReceiveBeginPlay`)
  (`|ExecutionSequence`
    (:`then_0`
      (if (`self.IsLocalPlayerController`)
        (`EnhancedInputSubsystemInterface.AddMappingContext` (subsystem `EnhancedInputLocalPlayerSubsystem`) "/Game/Input/IMC_Default.IMC_Default" 0 (struct))
        (bind _returnvalue (`|SpawnActorFromClass` "/Game/Actor/BP_Cursor.BP_Cursor_C" (`KismetMathLibrary.MakeTransform` (0.0 0.0 0.0)) "AlwaysSpawn" "MultiplyWithRoot" null null))
        (set `self.Cursor` _returnvalue)))
    (:`then_1`
      (bind _ascharacter (cast `Character` (`self.K2_GetPawn`)))
      (bind _output_get (set `self.ControlledCharacter` _ascharacter))
      (`|ExecutionSequence`
        (:`then_0`
          (add `self.OnActorBeginOverlap` _output_get (`|CreateDelegate` :!event `OnCharacterBeginOverlap`))
          (`/Game/FunctionLibrary/BP_FunctionLib_Event.Bind to Lua State Reload` self)
          (set `self.bShowMouseCursor` true)
          (`self.SetActorTickEnabled` true))
        (:`then_1`
          ;[1 1 1] TODO: currently doesn't do anything
          (bind _asbpi_gameplay_stat (cast `/Game/Interfaces/BPI_GameplayStat` (`self.ControlledCharacter`)))
          (bind _output_get_2 (set `self.CharacterStat` _asbpi_gameplay_stat))
          (`self.SetupMovementSpeed` _output_get_2))))))

(event `self.ReceiveTick`
  (params (DeltaSeconds :type "Float (single-precision)"))
  ;[1 1 1] Tick only run when char is valid (disabled by default)
  (`parent.ReceiveTick` DeltaSeconds)
  (message `/Game/Interfaces/BPI_CanAim.SetAimDirection` (`self.ControlledCharacter`) (`self.CalculateAimDirection`)))

(event `EnhancedInput|/Game/Input/IA_Move`
  (params (ActionValue :type "Vector2D Structure") (ElapsedSeconds :type "Float (double-precision)") (TriggeredSeconds :type "Float (double-precision)") (InputAction :type "InputAction Object Reference" :default "/Game/Input/IA_Move.IA_Move"))
  (bind (_x _y) (`KismetMathLibrary.BreakVector2D` ActionValue))
  (bind _controlledcharacter (`self.ControlledCharacter`))
  (:`Triggered`
    (`Pawn.AddMovementInput` _controlledcharacter (1.0 0.0 0.0) _x false)
    (`Pawn.AddMovementInput` _controlledcharacter (0.0 -1.0 0.0) _y false)
    (`KismetSystemLibrary.PrintString` "Hello")))

(event `EnhancedInput|/Game/Input/IA_Shoot`
  (params (ActionValue :type Boolean) (ElapsedSeconds :type "Float (double-precision)") (TriggeredSeconds :type "Float (double-precision)") (InputAction :type "InputAction Object Reference" :default "/Game/Input/IA_Shoot.IA_Shoot"))
  (:`Started`
    (message `/Game/Interfaces/BPI_CanEquipThings.InteractWithEquippedThing` (`self.ControlledCharacter`))))

(event `EnhancedInput|/Game/Input/IA_Reload`
  (params (ActionValue :type Boolean) (ElapsedSeconds :type "Float (double-precision)") (TriggeredSeconds :type "Float (double-precision)") (InputAction :type "InputAction Object Reference" :default "/Game/Input/IA_Reload.IA_Reload"))
  (:`Started`
    (message `/Game/Interfaces/BPI_CanEquipThings.SecondaryAction` (`self.ControlledCharacter`))))

(event `EnhancedInput|/Game/Input/IA_Jump`
  (params (ActionValue :type Boolean) (ElapsedSeconds :type "Float (double-precision)") (TriggeredSeconds :type "Float (double-precision)") (InputAction :type "InputAction Object Reference" :default "/Game/Input/IA_Jump.IA_Jump"))
  (:`Triggered`
    (`Character.Jump` (`self.ControlledCharacter`)))
  (:`Completed`
    (`Character.StopJumping` (`self.ControlledCharacter`))))

(event `OnCharacterBeginOverlap` :!signature `self.OnActorBeginOverlap`
  (params (OverlappedActor :type "Actor Object Reference") (OtherActor :type "Actor Object Reference"))
  (bind _asbpi_equippable (cast `/Game/Interfaces/BPI_Equippable` OtherActor))
  (message `/Game/Interfaces/BPI_CanEquipThings.EquipThing` (`self.ControlledCharacter`) _asbpi_equippable))

(event `EnhancedInput|/Game/Input/IA_Unequip`
  (params (ActionValue :type Boolean) (ElapsedSeconds :type "Float (double-precision)") (TriggeredSeconds :type "Float (double-precision)") (InputAction :type "InputAction Object Reference" :default "/Game/Input/IA_Unequip.IA_Unequip"))
  (:`Started`
    (message `/Game/Interfaces/BPI_CanEquipThings.UnequipThing` (`self.ControlledCharacter`))))

(event `EnhancedInput|/Game/Input/IA_LuaStateReload`
  (params (ActionValue :type Boolean) (ElapsedSeconds :type "Float (double-precision)") (TriggeredSeconds :type "Float (double-precision)") (InputAction :type "InputAction Object Reference" :default "/Game/Input/IA_LuaStateReload.IA_LuaStateReload"))
  (:`Started`
    (`LuaBlueprintFunctionLibrary.LuaStateReload` "/Game/Core/BP_LuaState_Gameplay.BP_LuaState_Gameplay_C")
    (`/Game/FunctionLibrary/BP_FunctionLib_Event.DispatchLuaStateReloadEvent`)))

(event `/Game/FunctionLibrary/BPI_EventListener.OnLuaStateReloaded`
  (`self.SetupMovementSpeed` (`self.CharacterStat`)))

(event `self.K2_ToggleDebug`
  (`/Engine/EditorBlueprintResources/StandardMacros.FlipFlop`
    (:`A`
      (`/Game/FunctionLibrary/BP_FunctionLib_Debug.EnableDebug`))
    (:`B`
      (`/Game/FunctionLibrary/BP_FunctionLib_Debug.DisableDebug`))))

(fn `CalculateAimDirection`
  (returns (ReturnValue :type "Vector Structure"))
  (bind (_returnvalue_x _returnvalue_y) (`KismetMathLibrary.BreakVector` (- (`self.K2_GetActorLocation` (`self.Cursor`)) (`self.K2_GetActorLocation` (`self.ControlledCharacter`)))))
  (return (`KismetMathLibrary.Normal` (`KismetMathLibrary.MakeVector` _returnvalue_x _returnvalue_y))))

(fn `SetupMovementSpeed`
  (params (Target :type "/Game/Interfaces/BPI_GameplayStat Interface"))
  (bind _returnvalue (`/Game/FunctionLibrary/BP_FunctionLib_Stat.GetStat` Target "SPEED"))
  (set `self.CurrentMoveSpeed` _returnvalue))

(fn `UserConstructionScript`)