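; BP_Cursor is an actor that follows the mouse pointer in the world, acting as a cursor on the ground plane.
; Each Tick it deprojects the first player controller's mouse position into a world ray, intersects that ray with the Z=0 plane, and moves the actor there without sweeping.
; The intersection is computed analytically, with no trace, so it ignores terrain and other geometry.
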(event `self.ReceiveTick`
  (params (DeltaSeconds :type "Float (single-precision)"))
  (bind (_worldlocation _worlddirection) (`PlayerController.DeprojectMousePositionToWorld` (`GameplayStatics.GetPlayerController` 0)))
  (`parent.ReceiveTick` DeltaSeconds)
  (`self.K2_SetActorLocation` (+ _worldlocation (* (* _worlddirection (/ (.z _worldlocation) (.z _worlddirection))) -1.0))))

(fn `UserConstructionScript`
  (`parent.UserConstructionScript`))