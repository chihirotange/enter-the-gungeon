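; Projectile actor that flies in a straight line and damages the first overlapped actor other than its instigator.
; BeginPlay normalizes Velocity into a direction and reads speed and lifespan through getter functions.
; Tick moves it manually by world offset without sweep, instead of using a movement component.
; Sphere overlap sends OnDamagedMessage with GetDamage's value, then destroys the actor; GetObjectPoolID returns None.
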(event `self.ReceiveBeginPlay`
  (`parent.ReceiveBeginPlay`)
  (set `self.Velocity` (`KismetMathLibrary.Normal` (`self.Velocity`)))
  (bind _returnvalue (`/Game/FunctionLibrary/BP_FunctionLib_Stat.GetSpeed` self))
  (set `self.Speed` _returnvalue)
  (bind _returnvalue_2 (`/Game/FunctionLibrary/BP_FunctionLib_Stat.GetLifeSpan` self))
  (`self.SetLifeSpan` _returnvalue_2))

(event `self.ReceiveTick`
  (params (DeltaSeconds :type "Float (single-precision)"))
  (`parent.ReceiveTick` DeltaSeconds)
  (`self.K2_AddActorWorldOffset` (* (* (`self.Velocity`) (`self.Speed`)) DeltaSeconds)))

(event `self.Sphere.OnComponentBeginOverlap`
  (params (OverlappedComponent :type "PrimitiveComponent Object Reference") (OtherActor :type "Actor Object Reference") (OtherComp :type "PrimitiveComponent Object Reference") (OtherBodyIndex :type Integer) (bFromSweep :type Boolean) (SweepResult :type "HitResult Structure (by ref)"))
  (if (!= OtherActor (`self.Instigator`))
    (bind _returnvalue (`/Game/FunctionLibrary/BP_FunctionLib_Stat.GetDamage` self))
    (message `/Game/Interfaces/BPI_Gameplay_Damageable.OnDamaged` OtherActor _returnvalue)
    (`self.K2_DestroyActor`)))

(fn `GetObjectPoolID`
  (returns (ID :type Name))
  (return "None"))

(fn `UserConstructionScript`
  (`parent.UserConstructionScript`))