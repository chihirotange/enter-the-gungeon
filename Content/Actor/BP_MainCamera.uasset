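; Main camera actor that follows the player's controlled pawn in X and Y at a fixed height.
; Setup reads a LENGTH stat to set the height, camera Z offset and ortho width, then becomes the view target and enables tick once a pawn is found.
; Setup runs on BeginPlay and again whenever the Lua state reloads, refreshing the stat-driven values.
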(event `self.ReceiveBeginPlay`
  (`parent.ReceiveBeginPlay`)
  (`/Game/FunctionLibrary/BP_FunctionLib_Event.Bind to Lua State Reload` self)
  (`self.Setup`))

(event `/Game/FunctionLibrary/BPI_EventListener.OnLuaStateReloaded`
  (`self.Setup`))

(event `self.ReceiveTick`
  (params (DeltaSeconds :type "Float (single-precision)"))
  (`parent.ReceiveTick` DeltaSeconds)
  (`self.K2_SetActorLocation` (`KismetMathLibrary.MakeVector` (.x (`self.K2_GetActorLocation` (`self.ControlledPawn`))) (.y (`self.K2_GetActorLocation` (`self.ControlledPawn`))) (`self.Height`))))

(fn `GetID`
  (returns (ID :type Name))
  (return (`self.ID`)))

(fn `Setup`
  (bind _returnvalue (`GameplayStatics.GetPlayerController` 0))
  (bind _returnvalue_2 (`Controller.K2_GetPawn` _returnvalue))
  (bind _returnvalue_3 (`/Game/FunctionLibrary/BP_FunctionLib_Stat.GetStat` self "LENGTH"))
  (set `self.Height` _returnvalue_3)
  (`SceneComponent.K2_SetRelativeLocation` (`self.CameraComponent`) (`KismetMathLibrary.MakeVector` 0.0 0.0 _returnvalue_3) false false)
  (`CameraComponent.SetOrthoWidth` (`self.CameraComponent`) _returnvalue_3)
  ;[1 1 1] TODO: improve?
  (`/Engine/EditorBlueprintResources/StandardMacros.IsValid` _returnvalue
    (:`Is Valid`
      (`PlayerController.SetViewTargetWithBlend` _returnvalue self 0.0 "VTBlend_Linear" 0.0 false)
      (`/Engine/EditorBlueprintResources/StandardMacros.IsValid` _returnvalue_2
        (:`Is Valid`
          (set `self.ControlledPawn` _returnvalue_2)
          (`self.SetActorTickEnabled` true))))))

(fn `UserConstructionScript`)