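; BP_AiChan is a networked character Blueprint with health, jumping, an orthographic spring-arm camera and an equipment slot.
; Camera and movement values come from stat lookups, applied on BeginPlay and reapplied when the Lua state reloads.
; Equipping runs through a server RPC, and the RepNotify attaches the item to EquipSlot.
; Aiming rotates that slot locally and on the server, snapping controller yaw forward or backward; zero HP destroys the actor.
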(event `self.ReceiveBeginPlay`
  (`parent.ReceiveBeginPlay`)
  (`self.SetupStats`)
  (add `/Game/ActorComponent/HealthComponent.OnHPReachedZero` (`self.HealthComponent`) (delegate `OnDead`)))

(event `OnDead`
  (`self.K2_DestroyActor`))

(event `SetupStats`
  (`self.SetupArmLength`)
  (`self.SetupJumpStat`))

(event `/Game/FunctionLibrary/BPI_EventListener.OnLuaStateReloaded`
  (`parent.OnLuaStateReloaded`)
  (`self.SetupStats`))

(event `/Game/Interfaces/BPI_Gameplay_Damageable.OnDamaged`
  (params (Damage :type Integer64))
  (`/Game/ActorComponent/HealthComponent.OnDamaged` (`self.HealthComponent`) Damage))

(event `/Game/Interfaces/BPI_CanEquipThings.EquipThing`
  (params (Thing :type "/Game/Interfaces/BPI_Equippable Interface"))
  ;[1 1 1] TODO: validation
  (`self.Server_EquipThing` Thing))

(event `Server_EquipThing`
  (params (Thing :type "/Game/Interfaces/BPI_Equippable Interface"))
  (set `self.CurrentlyEquippedThing` Thing))

(event `/Game/Interfaces/BPI_CanAim.SetAimDirection`
  (params (Direction :type "Vector Structure"))
  (`self.Server_SetAimDirection` Direction)
  (`SceneComponent.K2_SetWorldRotation` (`self.EquipSlot`) (`KismetMathLibrary.MakeRotFromX` Direction) false false)
  (`Controller.SetControlRotation` (`self.GetController`) (`KismetMathLibrary.MakeRotator` 0.0 0.0 (`KismetMathLibrary.SelectFloat` 0.0 180.0 (> (`KismetMathLibrary.Dot_VectorVector` (`KismetMathLibrary.Vector_Forward`) Direction) 0.0)))))

(event `Server_SetAimDirection`
  (params (AimDirection :type "Vector Structure"))
  (`SceneComponent.K2_SetWorldRotation` (`self.EquipSlot`) (`KismetMathLibrary.MakeRotFromX` AimDirection) false false))

(fn `OnRep_CurrentlyEquippedThing`
  (bind _asactor (cast `Actor` (`KismetSystemLibrary.Conv_InterfaceToObject` (`self.CurrentlyEquippedThing`))))
  (`/Game/Interfaces/BPI_Equippable.OnEquipped` (`self.CurrentlyEquippedThing`) self)
  (`self.K2_AttachToComponent` _asactor (`self.EquipSlot`) "None" "SnapToTarget" "SnapToTarget" "SnapToTarget" false))

(fn `SetupArmLength`
  (bind _returnvalue (`/Game/FunctionLibrary/BP_FunctionLib_Stat.Get Stat by ID` "MAIN_CAMERA" "LENGTH"))
  (set `SpringArmComponent.TargetArmLength` _returnvalue (`self.SpringArm`))
  (`CameraComponent.SetOrthoWidth` (`self.Camera`) _returnvalue))

(fn `SetupJumpStat`
  (`|ExecutionSequence`
    (:`then_0`
      (bind _returnvalue (`/Game/FunctionLibrary/BP_FunctionLib_Stat.GetStat` self "JUMP_VELOCITY"))
      (set `CharacterMovementComponent.JumpZVelocity` _returnvalue (`self.CharacterMovement`)))
    (:`then_1`
      (bind _returnvalue_2 (`/Game/FunctionLibrary/BP_FunctionLib_Stat.GetStat` self "AIR_CONTROL"))
      (set `CharacterMovementComponent.AirControl` _returnvalue_2 (`self.CharacterMovement`)))
    (:`then_2`
      (bind _returnvalue_3 (`/Game/FunctionLibrary/BP_FunctionLib_Stat.GetStat` self "GRAVITY_SCALE"))
      (set `CharacterMovementComponent.GravityScale` _returnvalue_3 (`self.CharacterMovement`)))))

(fn `UserConstructionScript`
  (`parent.UserConstructionScript`))