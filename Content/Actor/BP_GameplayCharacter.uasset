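; BP_GameplayCharacter is a gameplay character Blueprint that takes its walk speed from a stat and exposes its ID and Team through getters.
; On BeginPlay it binds to Lua state reload and runs SetupMoveSpeed, which copies the SPEED stat into CharacterMovement's MaxWalkSpeed.
; Each Lua reload re-applies that speed, so stat changes from reloaded scripts can take effect during play, and EndPlay removes the binding.
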(event `self.ReceiveBeginPlay`
  (`parent.ReceiveBeginPlay`)
  (`|ExecutionSequence`
    (:`then_0`
      (`/Game/FunctionLibrary/BP_FunctionLib_Event.Bind to Lua State Reload` self))
    (:`then_1`
      (`self.SetupMoveSpeed`))))

(event `/Game/FunctionLibrary/BPI_EventListener.OnLuaStateReloaded`
  (`self.SetupMoveSpeed`))

(event `self.ReceiveEndPlay`
  (params (EndPlayReason :type "EEndPlayReason Enum" :default "Destroyed"))
  (`parent.ReceiveEndPlay` EndPlayReason)
  (`/Game/FunctionLibrary/BP_FunctionLib_Event.UnbindToLuaStateReload` self))

(fn `GetID`
  (returns (ID :type Name))
  (return (`self.ID`)))

(fn `GetTeam`
  (returns (Team :type "ETeam Enum"))
  (return (`self.Team`)))

(fn `SetupMoveSpeed`
  (bind _returnvalue (`/Game/FunctionLibrary/BP_FunctionLib_Stat.GetStat` self "SPEED"))
  (set `CharacterMovementComponent.MaxWalkSpeed` _returnvalue (`self.CharacterMovement`)))

(fn `UserConstructionScript`)