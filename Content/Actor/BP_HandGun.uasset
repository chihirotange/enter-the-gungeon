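; BP_HandGun is an equippable 2D handgun that spawns BP_Projectile from its muzzle.
; Trigger calls the server, which fires with a timer-based fire-rate cooldown, cancelling any reload, or starts a timed reload when empty; SecondaryAction also reloads.
; Magazine size, fire rate and reload time come from stat lookups, re-read on Lua state reload.
; Equipping disables sprite physics and collision and sets owner and instigator on authority; unequipping reverses this.
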(event `self.ReceiveBeginPlay`
  (`parent.ReceiveBeginPlay`)
  (`self.ReadStats`)
  (`/Game/FunctionLibrary/BP_FunctionLib_Event.Bind to Lua State Reload` self))

(event `/Game/Interfaces/BPI_Triggerable.Trigger`
  (`self.Server_Trigger`))

(event `Server_Trigger`
  (if (> (`self.RemainingBullet`) 0)
    (if (`self.CanShoot`)
      (`self.Shoot`)
      (`self.StopReload`)
      ;[1 1 1] TODO: pool spawn
      (set `self.CanShoot` false)
      (`KismetSystemLibrary.K2_SetTimerDelegate` (delegate `OnCanShootAgain`) (`self.Firerate`)))
    (else
      ;[1 1 1] reload
      (`/Game/Interfaces/BPI_Triggerable.SecondaryAction`))))

(event `OnCanShootAgain`
  (set `self.CanShoot` true))

(event `/Game/Interfaces/BPI_Equippable.OnEquipped`
  (params (Instigator :type "Pawn Object Reference"))
  (`PrimitiveComponent.SetSimulatePhysics` (`self.PaperSprite`) false)
  ;[1 1 1] have to set this or this actor wont be able to be attached to another actor
  (`PrimitiveComponent.SetCollisionEnabled` (`self.PaperSprite`) "NoCollision")
  (`/Game/Macro/Macro_Networking.SwitchLocalRole`
    (:`Authority`
      (set `self.Instigator` Instigator)
      (`self.SetOwner` (`self.Instigator`)))))

(event `/Game/Interfaces/BPI_Equippable.OnUnequipped`
  (`PrimitiveComponent.SetCollisionEnabled` (`self.PaperSprite`) "PhysicsOnly")
  (`PrimitiveComponent.SetSimulatePhysics` (`self.PaperSprite`) true)
  (`/Game/Macro/Macro_Networking.SwitchLocalRole`
    (:`Authority`
      (set `self.Instigator` null)
      (`self.SetOwner` null))))

(event `/Game/FunctionLibrary/BPI_EventListener.OnLuaStateReloaded`
  (`self.ReadStats`))

(event `/Game/Interfaces/BPI_Triggerable.SecondaryAction`
  (if (not (`self.IsReloading`))
    (set `self.IsReloading` true)
    (bind _returnvalue (`KismetSystemLibrary.K2_SetTimerDelegate` (delegate `OnReloadCompleted`) (`self.ReloadTime`)))
    (set `self.ReloadHandler` _returnvalue)))

(event `OnReloadCompleted`
  (set `self.RemainingBullet` (`self.MagazineSize`))
  (`KismetSystemLibrary.PrintString` "Reloaded")
  (set `self.IsReloading` false))

(fn `ReadStats`
  (`|ExecutionSequence`
    (:`then_0`
      (bind _returnvalue (`/Game/FunctionLibrary/BP_FunctionLib_Stat.GetIntStat` self "BULLET"))
      (bind _output_get (set `self.RemainingBullet` _returnvalue))
      (set `self.MagazineSize` _output_get)
      (bind _returnvalue_2 (`/Game/FunctionLibrary/BP_FunctionLib_Stat.GetStat` self "FIRERATE"))
      (set `self.Firerate` _returnvalue_2))
    (:`then_1`
      (bind _returnvalue_3 (`/Game/FunctionLibrary/BP_FunctionLib_Stat.GetStat` self "RELOAD_TIME"))
      (set `self.ReloadTime` _returnvalue_3))))

(fn `Shoot`
  (bind _returnvalue (`self.GetInstigator`))
  (bind _returnvalue_2 (`SceneComponent.K2_GetComponentToWorld` (`self.Muzzle`)))
  (`/Engine/EditorBlueprintResources/StandardMacros.DecrementInt` (`self.RemainingBullet`)
    (:`  `
      (`|SpawnActorFromClass` "/Game/Actor/BP_Projectile.BP_Projectile_C" _returnvalue_2 "AlwaysSpawn" "MultiplyWithRoot" _returnvalue (`KismetMathLibrary.GetForwardVector` (.rotation _returnvalue_2)) _returnvalue))))

(fn `StopReload`
  (`KismetSystemLibrary.K2_ClearAndInvalidateTimerHandle` (`self.ReloadHandler`))
  (set `self.IsReloading` false))

(fn `UserConstructionScript`)