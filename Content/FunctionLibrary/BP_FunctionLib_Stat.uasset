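; Blueprint function library that reads actor stats and the camera spring arm length from the gameplay Lua state.
; GetStat passes an actor's uppercased ID and a stat key to the Lua get_stat function.
; Typed wrappers convert the results for max HP, speed, damage and lifespan, and unpack the jump table into velocity, air control and gravity scale.
; Camera arm length comes from a separate get_camera_info call.
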(fn `Get Max HP`
  (params (Actor :type "/Game/Interfaces/BPI_GameplayStat Interface"))
  (returns (ReturnValue :type Integer64))
  (bind _returnvalue (`self.GetStat` Actor "HP"))
  (return (`LuaBlueprintFunctionLibrary.Conv_LuaValueToInt64` _returnvalue)))

(fn `GetCameraArmLength`
  (returns (ReturnValue :type "Float (double-precision)"))
  (bind _returnvalue (`LuaBlueprintFunctionLibrary.LuaGlobalCall` null "/Game/Core/BP_LuaState_Gameplay.BP_LuaState_Gameplay_C" "get_camera_info" (`|MakeArray` (make `LuaValue` "String" false 0 0.0 "SPRING_ARM_LENGTH"))))
  (return (`LuaBlueprintFunctionLibrary.Conv_LuaValueToFloat` _returnvalue)))

(fn `GetDamage`
  (params (self2 :type "/Game/Interfaces/BPI_GameplayStat Interface"))
  (returns (ReturnValue :type Integer64))
  (bind _returnvalue (`self.GetStat` self2 "DAMAGE"))
  (return (`LuaBlueprintFunctionLibrary.Conv_LuaValueToInt64` _returnvalue)))

(fn `GetJumpStat`
  (params (self2 :type "/Game/Interfaces/BPI_GameplayStat Interface"))
  (returns (Velocity :type "Float (single-precision)") (`Air Control` :type "Float (double-precision)") (GravityScale :type "Float (double-precision)"))
  (bind _returnvalue (`self.GetStat` self2 "JUMP_STAT"))
  (return (`LuaBlueprintFunctionLibrary.Conv_LuaValueToFloat` (`LuaBlueprintFunctionLibrary.LuaTableGetField` _returnvalue "VELOCITY")) (`LuaBlueprintFunctionLibrary.Conv_LuaValueToFloat` (`LuaBlueprintFunctionLibrary.LuaTableGetField` _returnvalue "AIR_CONTROL")) (`LuaBlueprintFunctionLibrary.Conv_LuaValueToFloat` (`LuaBlueprintFunctionLibrary.LuaTableGetField` _returnvalue "GRAVITY_SCALE"))))

(fn `GetLifeSpan`
  (params (self2 :type "/Game/Interfaces/BPI_GameplayStat Interface"))
  (returns (ReturnValue :type "Float (single-precision)"))
  (bind _returnvalue (`self.GetStat` self2 "LIFESPAN"))
  (return (`LuaBlueprintFunctionLibrary.Conv_LuaValueToFloat` _returnvalue)))

(fn `GetSpeed`
  (params (self2 :type "/Game/Interfaces/BPI_GameplayStat Interface"))
  (returns (ReturnValue :type "Float (single-precision)"))
  (bind _returnvalue (`self.GetStat` self2 "SPEED"))
  (return (`LuaBlueprintFunctionLibrary.Conv_LuaValueToFloat` _returnvalue)))

(fn `GetStat`
  (params (self2 :type "/Game/Interfaces/BPI_GameplayStat Interface") (SourceString :type String))
  (returns (ReturnValue :type "LuaValue Structure"))
  (bind _id (`/Game/Interfaces/BPI_GameplayStat.GetID` self2))
  (bind _returnvalue (`LuaBlueprintFunctionLibrary.LuaGlobalCall` null "/Game/Core/BP_LuaState_Gameplay.BP_LuaState_Gameplay_C" "get_stat" (`|MakeArray` (make `LuaValue` "String" false 0 0.0 (`KismetStringLibrary.ToUpper` (`KismetStringLibrary.Conv_NameToString` _id))) (make `LuaValue` "String" false 0 0.0 SourceString))))
  (return _returnvalue))