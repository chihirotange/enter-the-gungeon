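; Blueprint function library for team checks, providing GetAttitude to resolve how one actor regards another.
; It returns Neutral unless both actors implement BPI_Team, then compares the teams they report through GetTeamMessage.
; A first actor on the NEUTRAL team yields Neutral; otherwise matching teams yield Friendly and differing teams Hostile.
; The check is asymmetric, as a neutral second actor reads as Hostile to a non-neutral first.
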(fn `GetAttitude`
  (params (FirstActor :type "Actor Object Reference") (SecondActor :type "Actor Object Reference"))
  (returns (Attitude :type "ETeamAttitude Enum"))
  (locals (SecondActorTeam :type "ETeam Enum" :default "TEAM_NEUTRAL"))
  (`|ExecutionSequence`
    (:`then_0`
      (if (not (and (`KismetSystemLibrary.DoesImplementInterface` (`local.FirstActor`) "/Game/Interfaces/BPI_Team.BPI_Team_C") (`KismetSystemLibrary.DoesImplementInterface` (`local.SecondActor`) "/Game/Interfaces/BPI_Team.BPI_Team_C")))
        (return "Neutral")))
    (:`then_1`
      (bind _team (message `/Game/Interfaces/BPI_Team.GetTeam` (`local.SecondActor`)))
      (set `local.SecondActorTeam` _team)
      (bind _team_2 (message `/Game/Interfaces/BPI_Team.GetTeam` (`local.FirstActor`)))
      (if (`|EnumEquality` _team_2 "TEAM_NEUTRAL")
        (return "Neutral")
        (elif (`|EnumEquality` _team_2 (`local.SecondActorTeam`))
          (return "Friendly")
          (else
            (return "Hostile")))))))